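; BP_PrimaryTest is a functional test that checks the player's first-person character can use its weapon's primary action.
; StartTest caches the player character, and Tick retries that lookup while the reference is invalid.
; Each tick pushes the character forward; once a current weapon exists, it sends the primary-pressed message.
; The test then finishes as succeeded immediately, without verifying the weapon's response.
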(event EventTick
  (params (DeltaSeconds :type Float%20%28single-precision%29))
  (Utilities|IsValid (Variables|Default|GetFirstPersonCharacter)
    (:Is%20Valid
      (Pawn|Input|AddMovementInput (Variables|Default|GetFirstPersonCharacter) (Transformation|GetActorForwardVector (Variables|Default|GetFirstPersonCharacter)) 1.0 false)
      (Utilities|IsValid (Variables|/Script/WeaponSystem_Team7.WeaponSystem_Team7Character|GetCurrentWeapon (Variables|Default|GetFirstPersonCharacter))
        (:Is%20Valid
          (Class|WeaponBPI|OnPrimaryPressed(Message) (Variables|/Script/WeaponSystem_Team7.WeaponSystem_Team7Character|GetCurrentWeapon (Variables|Default|GetFirstPersonCharacter)))
          (Class|FunctionalTest|FinishTest "Succeeded" "Using Primary"))))
    (:Is%20Not%20Valid
      (bind _asfirst_person_character (Utilities|Casting|CastToFirstPersonCharacter (Game|GetPlayerCharacter 0)))
      (Variables|Default|SetFirstPersonCharacter _asfirst_person_character))))

(event EventStartTest
  (bind _asfirst_person_character (Utilities|Casting|CastToFirstPersonCharacter (Game|GetPlayerCharacter 0)))
  (Variables|Default|SetFirstPersonCharacter _asfirst_person_character))

(fn ConstructionScript)