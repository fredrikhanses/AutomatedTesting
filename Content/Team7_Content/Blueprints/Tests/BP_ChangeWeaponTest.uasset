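; Automated functional test that checks the player's FirstPersonCharacter can change weapons.
; It caches player character 0 and its current weapon at test start, retrying on Tick while either reference is missing.
; Each tick it pushes the character forward and, once a weapon is recorded, requests a random weapon change, succeeding when the current weapon differs.
; No explicit failure result is reported.
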(event EventTick
  (params (DeltaSeconds :type Float%20%28single-precision%29))
  (Utilities|IsValid (Variables|Default|GetFirstPersonCharacter)
    (:Is%20Valid
      (Pawn|Input|AddMovementInput (Variables|Default|GetFirstPersonCharacter) (Transformation|GetActorForwardVector (Variables|Default|GetFirstPersonCharacter)) 1.0 false)
      (Utilities|IsValid (Variables|/Script/WeaponSystem_Team7.WeaponSystem_Team7Character|GetCurrentWeapon (Variables|Default|GetFirstPersonCharacter))
        (:Is%20Valid
          (Utilities|IsValid (Variables|Default|GetLastWeapon)
            (:Is%20Valid
              (Class|WeaponSystemTeam7Character|ChangeWeapon (Variables|Default|GetFirstPersonCharacter) (Math|Random|RandomInteger 3))
              (if (not (== (Variables|/Script/WeaponSystem_Team7.WeaponSystem_Team7Character|GetCurrentWeapon (Variables|Default|GetFirstPersonCharacter)) (Variables|Default|GetLastWeapon)))
                (Class|FunctionalTest|FinishTest "Succeeded" "Changing Weapon")))
            (:Is%20Not%20Valid
              (bind _asfirst_person_character (Utilities|Casting|CastToFirstPersonCharacter (Game|GetPlayerCharacter 0) :!label _label))
              (Variables|Default|SetFirstPersonCharacter _asfirst_person_character)
              (Utilities|IsValid (Variables|Default|GetLastWeapon)
                (:Is%20Not%20Valid
                  (Variables|Default|SetLastWeapon (Variables|/Script/WeaponSystem_Team7.WeaponSystem_Team7Character|GetCurrentWeapon (Variables|Default|GetFirstPersonCharacter))))))))))
    (:Is%20Not%20Valid
      (goto _label))))

(event EventStartTest
  (bind _asfirst_person_character (Utilities|Casting|CastToFirstPersonCharacter (Game|GetPlayerCharacter 0)))
  (Variables|Default|SetFirstPersonCharacter _asfirst_person_character)
  (Utilities|IsValid (Variables|Default|GetLastWeapon)
    (:Is%20Not%20Valid
      (Variables|Default|SetLastWeapon (Variables|/Script/WeaponSystem_Team7.WeaponSystem_Team7Character|GetCurrentWeapon (Variables|Default|GetFirstPersonCharacter))))))

(fn ConstructionScript)